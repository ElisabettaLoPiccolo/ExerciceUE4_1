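; Sphere actor that changes its mesh color when an actor of a specified pawn class overlaps it.
; BeginPlay applies the default color, and begin overlap on the collision component picks a random RGB color.
; End overlap either restores the default or randomizes again, depending on RevertBackToDefault.
; ApplyColor creates a dynamic material instance on each call and sets the named vector parameter.
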(event OnComponentBeginOverlap(Collision)
  (params (OverlappedComponent :type Primitive%20Component%20Object%20Reference) (OtherActor :type Actor%20Object%20Reference) (OtherComp :type Primitive%20Component%20Object%20Reference) (OtherBodyIndex :type Integer) (bFromSweep :type Boolean) (SweepResult :type Hit%20Result%20Structure%20%28by%20ref%29))
  ;[1 1 1] Sphere Behaviour
  (CallFunction|ChangeColor OtherActor "/Game/Blueprints/MyPawn.MyPawn_C" true))

(event OnComponentEndOverlap(Collision)
  (params (OverlappedComponent :type Primitive%20Component%20Object%20Reference) (OtherActor :type Actor%20Object%20Reference) (OtherComp :type Primitive%20Component%20Object%20Reference) (OtherBodyIndex :type Integer))
  ;[1 1 1] Sphere Behaviour
  (CallFunction|ChangeColor OtherActor "/Game/Blueprints/MyPawn.MyPawn_C" (not (Variables|Default|GetrevertBackToDefault))))

(event EventBeginPlay
  ;[1 1 1] Init
  (bind _output_get (Variables|Default|SetsphereColor (Variables|Default|GetdefaultSphereColor)))
  (CallFunction|ApplyColor (Variables|Default|GetMaterialColorName) _output_get))

(fn ConstructionScript)

(fn ChangeColor
  (params (overlappedActor :type Actor%20Object%20Reference) (toCompareWith :type Actor%20Class%20Reference) (setToRandom :type Boolean))
  (if (== (Utilities|GetClass overlappedActor) toCompareWith)
    (bind _output_get (Variables|Default|SetsphereColor (Math|Color|SelectColor (CallFunction|GetRandomColor) (Variables|Default|GetdefaultSphereColor) setToRandom)))
    (CallFunction|ApplyColor (Variables|Default|GetMaterialColorName) _output_get)))

(fn GetRandomColor
  (return (Utilities|Struct|MakeLinearColor (Math|Random|RandomFloat) (Math|Random|RandomFloat) (Math|Random|RandomFloat) 1.0)))

(fn ApplyColor
  (params (MaterialParamName :type Name) (Color :type Linear%20Color%20Structure))
  (bind _returnvalue (Rendering|Material|CreateDynamicMaterialInstance (Variables|Default|GetStaticMesh) 0 0 "None" :!class /Script/Engine.PrimitiveComponent))
  (Rendering|Material|SetVectorParameterValue _returnvalue MaterialParamName Color :!class /Script/Engine.MaterialInstanceDynamic))